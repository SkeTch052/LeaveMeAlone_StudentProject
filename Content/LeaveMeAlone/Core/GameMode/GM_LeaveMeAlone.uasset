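; Game mode for LeaveMeAlone that runs the match countdown and ends the game when time runs out.
; A looping one-second timer decrements GameTime until it reaches zero, then clears itself.
; At zero it flags the player controller as paused, pauses the game, shows the WBP_TimeIsUp widget and switches to UI-only input with a visible cursor.
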(event `self.ReceiveBeginPlay`
  (bind _returnvalue (`KismetSystemLibrary.K2_SetTimerDelegate` (delegate `CustomTimer`) 1.0 true))
  (set `self.GameTimerHandle` _returnvalue))

(event `CustomTimer`
  (bind _output_get (set `self.Game Time` (- (`self.Game Time`) 1)))
  (if (== _output_get 0)
    (`KismetSystemLibrary.K2_ClearAndInvalidateTimerHandle` (`self.GameTimerHandle`))
    (bind _aspc_leave_me_alone (cast `/Game/LeaveMeAlone/Core/Controller/PC_LeaveMeAlone` (`GameplayStatics.GetPlayerController` 0)))
    (set `/Game/LeaveMeAlone/Core/Controller/PC_LeaveMeAlone.OnPause` true _aspc_leave_me_alone)
    (`GameplayStatics.SetGamePaused` true)
    (bind _returnvalue (`|CreateWidget` "/Game/LeaveMeAlone/Widgets/UI/WBP_TimeIsUp.WBP_TimeIsUp_C"))
    (`UserWidget.AddToViewport` _returnvalue 0)
    (`WidgetBlueprintLibrary.SetInputMode_UIOnlyEx` _aspc_leave_me_alone _returnvalue)
    (set `PlayerController.bShowMouseCursor` true _aspc_leave_me_alone)))

(event `self.ReceiveTick`
  (params (DeltaSeconds :type "Float (single-precision)")))

(fn `UserConstructionScript`)